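; Racing game mode that tracks vehicle race progress and runs card actions for the dash-vehicle racer.
; On BeginPlay it registers player 0's vehicle and shows the position HUD.
; Each Tick it rebuilds a score map for connected vehicles, weighting laps above checkpoints crossed.
; Card activation constructs the action class named in the card data and executes it on the instigating vehicle, with a helper for spawning action actors.
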(event `self.ReceiveBeginPlay`
  (bind _asbp_dash_vehicle (cast `/Game/DungeonsDash/Actors/Vehicles/BP_DashVehicle` (`GameplayStatics.GetPlayerPawn` 0)))
  (bind _output_get (set `self.Vehicle` _asbp_dash_vehicle))
  (`KismetArrayLibrary.Array_Add` (`self.ConnectedVehicles`) _output_get)
  (bind _returnvalue (`|CreateWidget` "/Game/DungeonsDash/UI/WBP_PosicionHUD.WBP_PosicionHUD_C"))
  (`UserWidget.AddToViewport` _returnvalue 0))

(event `self.ReceiveTick`
  (params (DeltaSeconds :type "Float (single-precision)"))
  (bind _scoresmap (`self.ScoresMap`))
  (`/Engine/EditorBlueprintResources/StandardMacros.IsValid` (`self.Vehicle`)
    (:`Is Valid`
      (`BlueprintMapLibrary.Map_Clear` _scoresmap)
      (for _array_element (`self.ConnectedVehicles`)
        (bind _progressscore (`self.GetVehicleProgressScore` _array_element))
        (`BlueprintMapLibrary.Map_Add` _scoresmap _array_element _progressscore)))))

(fn `GetVehicleProgressScore`
  (params (Vehicle :type "/Game/DungeonsDash/Actors/Vehicles/BP_DashVehicle Object Reference"))
  (returns (ProgressScore :type "Float (double-precision)"))
  (return (`KismetMathLibrary.Conv_IntToDouble` (+ (* (`/Game/DungeonsDash/Actors/Vehicles/BP_DashVehicle.laps` Vehicle) 1000) (* (`/Game/DungeonsDash/Actors/Vehicles/BP_DashVehicle.checkpointscrossed` Vehicle) 10)))))

(fn `ProcessCardActivation`
  (params (CardData :type "/Game/DungeonsDash/_Core/Data/Cards/DA_Card_Base Object Reference") (Instigator :type "/Game/DungeonsDash/Actors/Vehicles/BP_DashVehicle Object Reference"))
  (locals (GameModeRef :type "/Game/DungeonsDash/_Core/GameModes/GM_RacingGame Object Reference"))
  (set `local.GameModeRef` self)
  (bind _returnvalue (`|GenericCreateObject` (`/Game/DungeonsDash/_Core/Data/Cards/DA_Card_Base.CardActionClass` CardData)))
  (`/Game/DungeonsDash/Actors/CardActions/BP_Action_Base.ExecuteAction` _returnvalue Instigator null CardData))

(fn `SpawnActionActor`
  (params (ActorClass :type "Actor Class Reference") (SpawnTransform :type "Transform Structure"))
  (returns (SpawnedActor :type "Actor Object Reference"))
  (bind _returnvalue (`|SpawnActorFromClass` ActorClass SpawnTransform "AlwaysSpawn" "MultiplyWithRoot" null null))
  (return _returnvalue))

(fn `UserConstructionScript`)