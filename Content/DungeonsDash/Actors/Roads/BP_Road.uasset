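; BP_Road is a road actor that builds its geometry along the Road spline in the construction script, with no active gameplay logic.
; It splits the spline into fixed 1000-unit segments, adding a spline mesh component for each, so any leftover length at the end stays uncovered.
; Each segment takes local-space positions and directions at its two distances, scaling tangents by segment length to follow the curve.
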(fn `UserConstructionScript`
  (bind _road (`self.Road`))
  (for _index (range (`KismetMathLibrary.FTrunc` (/ (`SplineComponent.GetSplineLength` _road) 1000.0)))
    (bind _returnvalue (`AddComponent|NODE_AddSplineMeshComponent-1`))
    (bind _returnvalue_2 (* _index 1000))
    (bind _returnvalue_3 (* (+ _index 1) 1000))
    (`SplineMeshComponent.SetStartAndEnd` _returnvalue (`SplineComponent.GetLocationAtDistanceAlongSpline` _road (`KismetMathLibrary.Conv_IntToDouble` _returnvalue_2) "Local") (* (`SplineComponent.GetDirectionAtDistanceAlongSpline` _road (`KismetMathLibrary.Conv_IntToDouble` _returnvalue_2) "Local") 1000.0) (`SplineComponent.GetLocationAtDistanceAlongSpline` _road (`KismetMathLibrary.Conv_IntToDouble` _returnvalue_3) "Local") (* (`SplineComponent.GetDirectionAtDistanceAlongSpline` _road (`KismetMathLibrary.Conv_IntToDouble` _returnvalue_3) "Local") 1000.0) true)
    (`SceneComponent.K2_AttachToComponent` (`self.DefaultSceneRoot`) null "None" "KeepRelative" "KeepRelative" "KeepRelative" true)))