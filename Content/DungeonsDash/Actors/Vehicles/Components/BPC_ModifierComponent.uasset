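; Vehicle component that holds temporary gameplay modifiers: speed boost, stun and shield.
; ApplyModifier switches on the modifier type, sets the matching state from Intensity where relevant, and starts a timer for Duration.
; Each timer fires a Remove event that resets that state, with debug prints for turbo on and off.
; OnRep handlers exist for turbo, shield, stun, invincibility and shield hits but are empty, and no logic here sets invincibility.
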(event `Remove_SpeedBoost`
  (set `self.CurrentSpeedMultiplier` 1.0)
  (set `self.bIsTurboActive` false)
  (`KismetSystemLibrary.PrintString` "Turbo Des habilitado"))

(event `Remove_Stun`
  (set `self.bIsStunned` false))

(event `ApplyModifier`
  (params (ModifierType :type "/Game/DungeonsDash/_Core/Data/Enums/E_DashModifierType Enum" :default "NewEnumerator0") (Duration :type "Float (double-precision)") (Intensity :type "Float (double-precision)"))
  (switch `/Game/DungeonsDash/_Core/Data/Enums/E_DashModifierType` ModifierType
    (:`NewEnumerator0`
      (set `self.CurrentSpeedMultiplier` Intensity)
      (set `self.bIsTurboActive` true)
      (`KismetSystemLibrary.K2_SetTimerDelegate` (delegate `Remove_SpeedBoost`) Duration)
      (`KismetSystemLibrary.PrintString` "Turbo habilitado"))
    (:`NewEnumerator2`
      (set `self.bIsStunned` true)
      (`KismetSystemLibrary.K2_SetTimerDelegate` (delegate `Remove_Stun`) Duration))
    (:`NewEnumerator3`
      (set `self.bHasShield` true)
      (set `self.ShieldHitsRemaining` (`KismetMathLibrary.FTrunc` Intensity))
      (`KismetSystemLibrary.K2_SetTimerDelegate` (delegate `Remove_Shield`) Duration))))

(event `Remove_Shield`
  (set `self.bHasShield` false)
  (set `self.ShieldHitsRemaining` 0))

(fn `OnRep_bHasShield`)

(fn `OnRep_bIsInvincible`)

(fn `OnRep_bIsStunned`)

(fn `OnRep_bIsTurboActive`)

(fn `OnRep_ShieldHitsRemaining`)