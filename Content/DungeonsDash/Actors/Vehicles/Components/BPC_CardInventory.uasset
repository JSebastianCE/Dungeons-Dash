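; Card inventory component for racing vehicles in DungeonsDash, holding cards up to a slot limit and firing a notification when one is added.
; Next and previous selection wrap around the slots, and using a card sends the selected index through a server request.
; That request removes the slot, then passes the card read at that index (after removal) and the owning vehicle to GM_RacingGame for activation.
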(event `Server_RequestUseCard`
  (params (CardIndex :type Integer))
  (if (`KismetArrayLibrary.Array_IsValidIndex` (`self.CardSlots`) CardIndex)
    (`KismetArrayLibrary.Array_Remove` (`self.CardSlots`) CardIndex)
    (bind _asgm_racing_game (cast `/Game/DungeonsDash/_Core/GameModes/GM_RacingGame` (`GameplayStatics.GetGameMode`)))
    (`/Game/DungeonsDash/_Core/GameModes/GM_RacingGame.ProcessCardActivation` _asgm_racing_game (`|GetArrayItem` (`self.CardSlots`) CardIndex) (`self.OwningVehicle`))))

(fn `AddCard`
  (params (CardData :type "/Game/DungeonsDash/_Core/Data/Cards/DA_Card_Base Object Reference"))
  (returns (Success :type Boolean))
  (if (< (`KismetArrayLibrary.Array_Length` (`self.CardSlots`)) (`self.MaxCardSlots`))
    (`KismetArrayLibrary.Array_Add` (`self.CardSlots`) CardData)
    (`self.OnCardAdded`)
    (return true)
    (else
      (return false))))

(fn `SelectNextCard`
  (set `self.SelectCardIndex` (mod (+ (`self.SelectCardIndex`) 1) (`KismetArrayLibrary.Array_Length` (`self.CardSlots`))))
  (return))

(fn `SelectPreviousCard`
  (bind _returnvalue (`KismetArrayLibrary.Array_Length` (`self.CardSlots`)))
  (set `self.SelectCardIndex` (mod (+ (- (`self.SelectCardIndex`) 1) _returnvalue) _returnvalue))
  (return))

(fn `UseCurrentCard`
  (`self.Server_RequestUseCard` (`self.SelectCardIndex`)))