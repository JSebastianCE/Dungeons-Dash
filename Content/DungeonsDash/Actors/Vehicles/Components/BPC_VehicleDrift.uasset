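; Vehicle component for BP_DashVehicle that adds kart-style drifting with a charged mini-turbo.
; While the drift button is held, Tick starts a drift if steering, speed and ground checks pass, raising the handling multiplier.
; Drift charge builds up to a cap until EndDrift, not called here, converts it into a forward boost message to the owner.
; Handling is not restored here, and debug prints remain throughout.
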(event `self.ReceiveTick`
  (params (DeltaSeconds :type "Float (single-precision)"))
  (bind _bisdrifting (`self.bIsDrifting`))
  (`|ExecutionSequence`
    (:`then_0`
      (if (and (not _bisdrifting) (`self.bDriftButtonHeld`))
        (`self.StartDrift`)))
    (:`then_1`
      (if _bisdrifting
        (`self.UpdateDrift` DeltaSeconds)))))

(fn `ActivateMiniTurbo`
  (bind _returnvalue (`KismetMathLibrary.MapRangeClamped` (`self.DriftCharge`) (`self.MiniTurboThreshold`) (`self.MaxDriftCharge`) 0.0 (`self.MiniTurboForce`)))
  (message `/Game/DungeonsDash/_Core/BlueprintInterfaces/BPI_VehicleEffects.ApplyForwardBoost` (`self.GetOwner`) _returnvalue)
  (`KismetSystemLibrary.PrintString` (`KismetStringLibrary.Concat_StrStr` "Furza Miniturbo" (`KismetStringLibrary.Conv_DoubleToString` _returnvalue)) true true (struct :`R` 1.0 :`G` 0.104429 :`B` 0.072911 :`A` 1.0)))

(fn `EndDrift`
  (`self.ActivateMiniTurbo`)
  (`KismetSystemLibrary.PrintString` "Activado")
  (set `self.bIsDrifting` false)
  (set `self.DriftCharge` 0.0))

(fn `StartDrift`
  (bind _asbp_dash_vehicle (cast `/Game/DungeonsDash/Actors/Vehicles/BP_DashVehicle` (`self.GetOwner`)))
  (bind _returnvalue (`ChaosVehicleMovementComponent.GetSteeringInput` (`WheeledVehiclePawn.VehicleMovementComponent` _asbp_dash_vehicle)))
  (bind _returnvalue_2 (>= (`KismetMathLibrary.Abs` _returnvalue) (`self.MinSteerForDrift`)))
  (bind _returnvalue_3 (> (`KismetMathLibrary.VSize` (`Actor.GetVelocity` _asbp_dash_vehicle)) (`self.MinSpeedForDrift`)))
  (bind _bisgrounded (`/Game/DungeonsDash/Actors/Vehicles/BP_DashVehicle.bIsGrounded` _asbp_dash_vehicle))
  (if (and _returnvalue_2 _returnvalue_3 _bisgrounded)
    (set `self.bIsDrifting` true)
    (set `self.DriftCharge` 0.0)
    (`KismetSystemLibrary.PrintString` "Esta Drifteando")
    (set `/Game/DungeonsDash/Actors/Vehicles/Components/BPC_ModifierComponent.CurrentHandlingMultiplier` 2.0 (`/Game/DungeonsDash/Actors/Vehicles/BP_DashVehicle.BPC_ModifierComponent` _asbp_dash_vehicle))
    (else
      (`KismetSystemLibrary.PrintString` (`KismetStringLibrary.Concat_StrStr` "isgrounded: " (`KismetStringLibrary.Conv_BoolToString` _bisgrounded)) true true (struct :`R` 1.0 :`G` 0.837572 :`A` 1.0) 0.0)
      (`KismetSystemLibrary.PrintString` (`KismetStringLibrary.Concat_StrStr` "Speeddrift" (`KismetStringLibrary.Conv_BoolToString` _returnvalue_3)) true true (struct :`R` 0.091566 :`G` 1.0 :`B` 0.118027 :`A` 1.0) 0.0)
      (`KismetSystemLibrary.PrintString` (`KismetStringLibrary.Concat_StrStr` "Steering" (`KismetStringLibrary.Conv_BoolToString` _returnvalue_2)) true true (struct :`R` 0.466087 :`G` 0.172382 :`A` 1.0) 0.0))))

(fn `UpdateDrift`
  (params (DeltaSeconds :type "Float (double-precision)"))
  (if (`self.bIsDrifting`)
    (bind _output_get (set `self.DriftCharge` (`KismetMathLibrary.FClamp` (+ (* DeltaSeconds (`self.DriftChargeRate`)) (`self.DriftCharge`)) 0.0 (`self.MaxDriftCharge`))))
    (`KismetSystemLibrary.PrintString` (`KismetStringLibrary.Concat_StrStr` "Carga de drift" (`KismetStringLibrary.Conv_DoubleToString` _output_get)) true true (struct :`R` 1.0 :`B` 0.803329 :`A` 1.0) 0.0)))