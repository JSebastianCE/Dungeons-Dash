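; Player-driven racing vehicle for Dungeons Dash with jump, drift, card actions and checkpoint-based laps.
; Enhanced Input feeds the vehicle movement and drift components, with the modifier component gating controls through stun and scaling steering.
; Boost and hit handlers apply mesh impulses; shields absorb hits, otherwise the car spins and is stunned.
; Includes debug keys, prints and a hardcoded test fireball; a downward trace gates jumping.
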(event `self.ReceiveTick`
  (params (DeltaSeconds :type "Float (single-precision)"))
  (`KismetSystemLibrary.PrintString` (`KismetStringLibrary.Conv_DoubleToString` (* (`KismetMathLibrary.VSize` (`self.GetVelocity`)) 0.036)) true true (struct :`G` 0.66 :`B` 1.0 :`A` 1.0) 2.0 "KM/H")
  (`self.CheckGrounded`))

(event `self.ReceiveBeginPlay`
  (`EnhancedInputSubsystemInterface.AddMappingContext` (pcsubsystem `EnhancedInputLocalPlayerSubsystem` (`GameplayStatics.GetPlayerController` 0)) "/Game/DungeonsDash/_Core/Input/IMC_VehicleControls.IMC_VehicleControls" 0 (struct))
  ;[0.2431 1 0.007689 0.5] Laps
  (bind _returnvalue (`|CreateWidget` "/Game/DungeonsDash/Actors/CheckPoints/UI_CheckPoints/WBP_HUD_Carrera.WBP_HUD_Carrera_C"))
  (`UserWidget.AddToViewport` _returnvalue 0))

(event `EnhancedInput|/Game/DungeonsDash/_Core/Input/Actions/IA_Accelerate`
  (params (ActionValue :type "Float (double-precision)") (ElapsedSeconds :type "Float (double-precision)") (TriggeredSeconds :type "Float (double-precision)") (InputAction :type "InputAction Object Reference" :default "/Game/DungeonsDash/_Core/Input/Actions/IA_Accelerate.IA_Accelerate"))
  (:`Triggered`
    (if (not (`/Game/DungeonsDash/Actors/Vehicles/Components/BPC_ModifierComponent.bIsStunned` (`self.BPC_ModifierComponent`))) :!label _label
      (`ChaosVehicleMovementComponent.SetThrottleInput` (`self.VehicleMovementComponent`) ActionValue)))
  (:`Completed`
    (goto _label)))

(event `EnhancedInput|/Game/DungeonsDash/_Core/Input/Actions/IA_Steer`
  (params (ActionValue :type "Float (double-precision)") (ElapsedSeconds :type "Float (double-precision)") (TriggeredSeconds :type "Float (double-precision)") (InputAction :type "InputAction Object Reference" :default "/Game/DungeonsDash/_Core/Input/Actions/IA_Steer.IA_Steer"))
  (:`Triggered`
    (if (not (`/Game/DungeonsDash/Actors/Vehicles/Components/BPC_ModifierComponent.bIsStunned` (`self.BPC_ModifierComponent`))) :!label _label_2
      (`ChaosVehicleMovementComponent.SetSteeringInput` (`self.VehicleMovementComponent`) (* ActionValue (`/Game/DungeonsDash/Actors/Vehicles/Components/BPC_ModifierComponent.CurrentHandlingMultiplier` (`self.BPC_ModifierComponent`))))))
  (:`Completed`
    (goto _label_2)))

(event `EnhancedInput|/Game/DungeonsDash/_Core/Input/Actions/IA_Jump`
  (params (ActionValue :type Boolean) (ElapsedSeconds :type "Float (double-precision)") (TriggeredSeconds :type "Float (double-precision)") (InputAction :type "InputAction Object Reference" :default "/Game/DungeonsDash/_Core/Input/Actions/IA_Jump.IA_Jump"))
  (bind _bpc_vehicledrift (`self.BPC_VehicleDrift`))
  (:`Started`
    (`self.TryJump`)
    (set `/Game/DungeonsDash/Actors/Vehicles/Components/BPC_VehicleDrift.bDriftButtonHeld` true _bpc_vehicledrift))
  (:`Completed`
    (set `/Game/DungeonsDash/Actors/Vehicles/Components/BPC_VehicleDrift.bDriftButtonHeld` false _bpc_vehicledrift)
    (`/Game/DungeonsDash/Actors/Vehicles/Components/BPC_VehicleDrift.EndDrift` _bpc_vehicledrift)))

(event `EnhancedInput|/Game/DungeonsDash/_Core/Input/Actions/IA_Brake`
  (params (ActionValue :type "Float (double-precision)") (ElapsedSeconds :type "Float (double-precision)") (TriggeredSeconds :type "Float (double-precision)") (InputAction :type "InputAction Object Reference" :default "/Game/DungeonsDash/_Core/Input/Actions/IA_Brake.IA_Brake"))
  (:`Triggered`
    (if (not (`/Game/DungeonsDash/Actors/Vehicles/Components/BPC_ModifierComponent.bIsStunned` (`self.BPC_ModifierComponent`))) :!label _label_3
      (`ChaosVehicleMovementComponent.SetBrakeInput` (`self.VehicleMovementComponent`) ActionValue)))
  (:`Completed`
    (goto _label_3)))

(event `EnhancedInput|/Game/DungeonsDash/_Core/Input/Actions/IA_Handbrake`
  (params (ActionValue :type Boolean) (ElapsedSeconds :type "Float (double-precision)") (TriggeredSeconds :type "Float (double-precision)") (InputAction :type "InputAction Object Reference" :default "/Game/DungeonsDash/_Core/Input/Actions/IA_Handbrake.IA_Handbrake"))
  (bind _vehiclemovementcomponent (`self.VehicleMovementComponent`))
  (:`Started`
    (`ChaosVehicleMovementComponent.SetHandbrakeInput` _vehiclemovementcomponent ActionValue))
  (:`Completed`
    (`ChaosVehicleMovementComponent.SetHandbrakeInput` _vehiclemovementcomponent false)))

(event `EnhancedInput|/Game/DungeonsDash/_Core/Input/Actions/IA_UseCard`
  (params (ActionValue :type Boolean) (ElapsedSeconds :type "Float (double-precision)") (TriggeredSeconds :type "Float (double-precision)") (InputAction :type "InputAction Object Reference" :default "/Game/DungeonsDash/_Core/Input/Actions/IA_UseCard.IA_UseCard"))
  (:`Started`
    (`KismetSystemLibrary.PrintString` "Tecla E presionad")
    (bind _asgm_racing_game (cast `/Game/DungeonsDash/_Core/GameModes/GM_RacingGame` (`GameplayStatics.GetGameMode`)))
    (bind _returnvalue (`|GenericCreateObject` "/Game/DungeonsDash/Actors/CardActions/BP_Action_Fireball.BP_Action_Fireball_C"))
    (`/Game/DungeonsDash/Actors/CardActions/BP_Action_Base.ExecuteAction` _returnvalue self _asgm_racing_game (`self.TestCardData`))))

(event `Key|C`
  (params (Key :type "Key Structure"))
  (bind _lastcheckpoint (`self.lastcheckpoint`))
  (:`Pressed`
    (`self.K2_SetActorTransform` (`KismetMathLibrary.MakeTransform` (`self.K2_GetActorLocation` _lastcheckpoint) (`self.K2_GetActorRotation` _lastcheckpoint)) false true)))

(event `finish`
  (bind _laps (`self.laps`))
  ;[1 0 0.9515 0.5] CheckPonts
  (if (== (`self.checkpointscrossed`) 7)
    (`/Engine/EditorBlueprintResources/StandardMacros.IncrementInt` _laps
      (:`  `
        (set `self.checkpointscrossed` 0)
        (if (>= _laps 1)
          (`KismetSystemLibrary.PrintString` "¡CARRERA TERMINADA!"))))
    (else
      (`KismetSystemLibrary.PrintString` "\"¡Vuelta inválida! Te saltaste checkpoints\""))))

(event `/Game/DungeonsDash/_Core/BlueprintInterfaces/BPI_VehicleEffects.ApplyForwardBoost`
  (params (BoostForce :type "Float (double-precision)"))
  (`PrimitiveComponent.AddImpulse` (`self.Mesh`) (* BoostForce (`self.GetActorForwardVector`)) "None" true)
  (`KismetSystemLibrary.PrintString` "SE USO LA INTEFAZ Forward Boost"))

(event `Key|One`
  (params (Key :type "Key Structure"))
  (:`Pressed`
    (`/Game/DungeonsDash/Actors/Vehicles/Components/BPC_ModifierComponent.ApplyModifier` (`self.BPC_ModifierComponent`) "NewEnumerator3" 10.0 2.0)
    (`KismetSystemLibrary.PrintString` "Se activo escudo ")))

(event `/Game/DungeonsDash/_Core/BlueprintInterfaces/BPI_VehicleEffects.ApplyExternalBoost`
  (params (ExternalBoostForce :type "Float (double-precision)") (Direction :type "Vector Structure"))
  (`PrimitiveComponent.AddImpulse` (`self.Mesh`) (* ExternalBoostForce (`self.GetActorForwardVector`)) "None" true)
  (`KismetSystemLibrary.PrintString` "SE USO LA INTEFAZ External Boost"))

(event `Key|Two`
  (params (Key :type "Key Structure"))
  (:`Pressed`
    (`self.ApplyHitImpulse` (0.0 1.0 0.0) 200.0)))

(event `/Game/DungeonsDash/_Core/BlueprintInterfaces/BPI_VehicleEffects.ApplyTemporaryControlLoss`
  (params (Duration :type "Float (double-precision)"))
  (`/Game/DungeonsDash/Actors/Vehicles/Components/BPC_ModifierComponent.ApplyModifier` (`self.BPC_ModifierComponent`) "NewEnumerator2" Duration 0.0)
  (`KismetSystemLibrary.PrintString` "Me estunearon"))

(event `/Game/DungeonsDash/_Core/BlueprintInterfaces/BPI_VehicleEffects.ApplyHitImpulse`
  (params (Direction :type "Vector Structure") (Force :type "Float (double-precision)"))
  (bind _bpc_modifiercomponent (`self.BPC_ModifierComponent`))
  (bind _mesh (`self.Mesh`))
  (if (`/Game/DungeonsDash/Actors/Vehicles/Components/BPC_ModifierComponent.bHasShield` _bpc_modifiercomponent)
    (bind _output_get (set `/Game/DungeonsDash/Actors/Vehicles/Components/BPC_ModifierComponent.ShieldHitsRemaining` (- (`/Game/DungeonsDash/Actors/Vehicles/Components/BPC_ModifierComponent.ShieldHitsRemaining` _bpc_modifiercomponent) 1) _bpc_modifiercomponent))
    (if (<= _output_get 0)
      (set `/Game/DungeonsDash/Actors/Vehicles/Components/BPC_ModifierComponent.bHasShield` false _bpc_modifiercomponent)
      (`KismetSystemLibrary.PrintString` "Sin escudos"))
    (else
      (`PrimitiveComponent.AddImpulse` _mesh (* Direction Force) "None" true)
      (`PrimitiveComponent.AddAngularImpulseInDegrees` _mesh (0.0 0.0 5000.0) "None" true)
      (message `/Game/DungeonsDash/_Core/BlueprintInterfaces/BPI_VehicleEffects.ApplyTemporaryControlLoss` self 2.0))))

(fn `CheckGrounded`
  (bind _returnvalue (`self.K2_GetActorLocation`))
  (bind (_outhit _returnvalue_2) (`KismetSystemLibrary.LineTraceSingle` :`Start` _returnvalue :`End` (- _returnvalue (0.0 0.0 300.0)) :`TraceChannel` "TraceTypeQuery1" :`DrawDebugType` "ForOneFrame"))
  (bind _output_get (set `self.bIsGrounded` _returnvalue_2))
  (`KismetSystemLibrary.PrintString` (`KismetStringLibrary.Conv_BoolToString` _output_get) true true (struct :`G` 0.66 :`B` 1.0 :`A` 1.0) 2.0 "Is Grounded"))

(fn `GetProjectileSpawnPoint`
  (returns (SpawnTransform :type "Transform Structure"))
  (return (`SceneComponent.K2_GetComponentToWorld` (`self.SpawnPuntoFuego`))))

(fn `ReceiveCard`
  (params (CardData :type "/Game/DungeonsDash/_Core/Data/Cards/DA_Card_Base Object Reference"))
  (returns (`bWasAdded ` :type Boolean))
  (bind _success (`/Game/DungeonsDash/Actors/Vehicles/Components/BPC_CardInventory.AddCard` (`self.BPC_CardInventory`) CardData))
  (return _success))

(fn `ResetJump`
  (set `self.bCanJump` true))

(fn `TryJump`
  (if (and (`self.bCanJump`) (`self.bIsGrounded`))
    (`PrimitiveComponent.AddImpulse` (`self.Mesh`) (`KismetMathLibrary.MakeVector` 0.0 0.0 (`self.JumpForce`)) "None" true)
    (set `self.bCanJump` false)
    (`KismetSystemLibrary.K2_SetTimer` null "ResetJump" (`self.JumpCooldown`))))

(fn `UserConstructionScript`)