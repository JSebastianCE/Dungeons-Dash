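; Base dash vehicle Blueprint that drives by pushing a physics sphere, using Enhanced Input.
; BeginPlay adds the vehicle mapping context for player 0; steering yaws the actor, scaled by Handling.
; Accelerate applies mass-independent force to the sphere along the actor's forward vector, scaled by Acceleration, and Tick clamps its velocity to MaxSpeed.
; Both input handlers print debug values.
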(event `self.ReceiveBeginPlay`
  (`EnhancedInputSubsystemInterface.AddMappingContext` (pcsubsystem `EnhancedInputLocalPlayerSubsystem` (`GameplayStatics.GetPlayerController` 0)) "/Game/DungeonsDash/_Core/Input/IMC_VehicleControls.IMC_VehicleControls" 0 (struct)))

(event `self.ReceiveTick`
  (params (DeltaSeconds :type "Float (single-precision)"))
  (bind _sphere (`self.Sphere`))
  (`PrimitiveComponent.SetPhysicsLinearVelocity` _sphere (`KismetMathLibrary.ClampVectorSize` (`SceneComponent.GetComponentVelocity` _sphere) 0.0 (`self.MaxSpeed`)) false "None"))

(event `EnhancedInput|/Game/DungeonsDash/_Core/Input/Actions/IA_Steer`
  (params (ActionValue :type "Float (double-precision)") (ElapsedSeconds :type "Float (double-precision)") (TriggeredSeconds :type "Float (double-precision)") (InputAction :type "InputAction Object Reference" :default "/Game/DungeonsDash/_Core/Input/Actions/IA_Steer.IA_Steer"))
  (bind _returnvalue (* ActionValue (`self.Handling`)))
  (:`Triggered`
    (`self.K2_AddActorLocalRotation` (`KismetMathLibrary.MakeRotator` 0.0 0.0 _returnvalue))
    (`KismetSystemLibrary.PrintString` (`KismetStringLibrary.Conv_DoubleToString` _returnvalue))))

(event `EnhancedInput|/Game/DungeonsDash/_Core/Input/Actions/IA_Accelerate`
  (params (ActionValue :type "Float (double-precision)") (ElapsedSeconds :type "Float (double-precision)") (TriggeredSeconds :type "Float (double-precision)") (InputAction :type "InputAction Object Reference" :default "/Game/DungeonsDash/_Core/Input/Actions/IA_Accelerate.IA_Accelerate"))
  (:`Triggered`
    (`PrimitiveComponent.AddForce` (`self.Sphere`) (* (`self.GetActorForwardVector`) (`self.Acceleration`) ActionValue) "None" true)
    (`KismetSystemLibrary.PrintString` (`KismetStringLibrary.Conv_DoubleToString` ActionValue))
    (`KismetSystemLibrary.PrintString` (`KismetStringLibrary.Conv_Vector3fToString` (`SceneComponent.GetComponentVelocity` (`self.Sphere`))))))

(fn `UserConstructionScript`)