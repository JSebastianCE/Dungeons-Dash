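; BP_Projectile_Base is a projectile actor, apparently a base class, that pushes the actors it overlaps.
; On HitBox overlap it sends an ApplyHitImpulse message to the other actor with a fixed force along the ProjectileMovement velocity direction.
; The blocking-hit handler skips the owner and casts to BP_DashVehicle but takes no further action.
; A delayed self-destroy is present but never runs.
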(event `self.HitBox.OnComponentBeginOverlap`
  (params (OverlappedComponent :type "PrimitiveComponent Object Reference") (OtherActor :type "Actor Object Reference") (OtherComp :type "PrimitiveComponent Object Reference") (OtherBodyIndex :type Integer) (bFromSweep :type Boolean) (SweepResult :type "HitResult Structure (by ref)"))
  (message `/Game/DungeonsDash/_Core/BlueprintInterfaces/BPI_VehicleEffects.ApplyHitImpulse` OtherActor (`KismetMathLibrary.Normal` (`MovementComponent.Velocity` (`self.ProjectileMovement`))) 1500.0))

(event `self.HitBox.OnComponentHit`
  (params (HitComponent :type "PrimitiveComponent Object Reference") (OtherActor :type "Actor Object Reference") (OtherComp :type "PrimitiveComponent Object Reference") (NormalImpulse :type "Vector Structure") (Hit :type "HitResult Structure (by ref)"))
  (if (not (== OtherActor (`self.GetOwner`)))
    (cast `/Game/DungeonsDash/Actors/Vehicles/BP_DashVehicle` OtherActor)))

(fn `UserConstructionScript`)