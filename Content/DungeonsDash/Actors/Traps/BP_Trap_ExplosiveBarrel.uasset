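; BP_Trap_ExplosiveBarrel is a trap actor that applies a modifier to dash vehicles that touch it.
; It arms itself after a short delay on BeginPlay, then its Sphere overlap ignores the owner and accepts only BP_DashVehicle.
; A hit applies one fixed modifier type through the vehicle's BPCModifierComponent, with zero duration and intensity.
; The graph ends on a brief delay, with no explosion or destroy logic.
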(event `self.ReceiveBeginPlay`
  (set `self.bArmed` false)
  (`KismetSystemLibrary.Delay` 1.5)
  (set `self.bArmed` true))

(event `self.Sphere.OnComponentBeginOverlap`
  (params (OverlappedComponent :type "PrimitiveComponent Object Reference") (OtherActor :type "Actor Object Reference") (OtherComp :type "PrimitiveComponent Object Reference") (OtherBodyIndex :type Integer) (bFromSweep :type Boolean) (SweepResult :type "HitResult Structure (by ref)"))
  (if (and (`self.bArmed`) (!= OtherActor (`self.GetOwner`)))
    (bind _asbp_dash_vehicle (cast `/Game/DungeonsDash/Actors/Vehicles/BP_DashVehicle` OtherActor))
    (`/Game/DungeonsDash/Actors/Vehicles/Components/BPC_ModifierComponent.ApplyModifier` (`/Game/DungeonsDash/Actors/Vehicles/BP_DashVehicle.BPC_ModifierComponent` _asbp_dash_vehicle) "NewEnumerator2" 0.0 0.0)
    (`KismetSystemLibrary.Delay` 0.2)))

(fn `UserConstructionScript`)