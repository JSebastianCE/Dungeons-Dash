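; Base card pickup that gives a fixed or randomly chosen card to an overlapping actor's inventory, with debug prints describing vehicles as the receivers.
; Sphere overlap checks for BPI_CardInventoryReceiver, gets a valid card from GetCardToGive and passes it through the interface.
; Only a successful receive deactivates the pickup, hiding its mesh and disabling collision, so a full inventory leaves it active.
; Respawnable pickups then set a timer, and RespawnPickup restores visibility and collision.
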(event `self.ReceiveBeginPlay`)

(event `self.SphereCollision.OnComponentBeginOverlap`
  (params (OverlappedComponent :type "PrimitiveComponent Object Reference") (OtherActor :type "Actor Object Reference") (OtherComp :type "PrimitiveComponent Object Reference") (OtherBodyIndex :type Integer) (bFromSweep :type Boolean) (SweepResult :type "HitResult Structure (by ref)"))
  (`KismetSystemLibrary.PrintString` (`KismetSystemLibrary.GetDisplayName` OtherActor))
  ;[0.159 0.9047 0.2705 0.502 10] VALIDAR PICKUP ACTIVO
  (if (`self.bIsActive`)
    ;[0.159 0.9047 0.2705 0.502 10] VALIDAR RECEPTOR DE CARTAS
    (if (`KismetSystemLibrary.DoesImplementInterface` OtherActor "/Game/DungeonsDash/_Core/BlueprintInterfaces/BPI_CardInventoryReceiver.BPI_CardInventoryReceiver_C")
      (`KismetSystemLibrary.PrintString` "Vehículo Detectado" true true (struct :`R` 0.307423 :`B` 1.0 :`A` 1.0))
      ;[0.6376 0.162 1 0.502 10] OBTENER CARTA DEL PICKUP
      (bind (_cardtogive _bhasvalidcard) (`self.GetCardToGive`))
      (if _bhasvalidcard
        (`KismetSystemLibrary.PrintString` (`KismetTextLibrary.Conv_TextToString` (`/Game/DungeonsDash/_Core/Data/Cards/DA_Card_Base.CardName` _cardtogive)) true true (struct :`R` 0.046866 :`G` 1.0 :`A` 1.0))
        ;[0.2193 0.9039 0.9792 0.5 10] ENTREGAR CARTA AL INVENTARIO
        (bind _bwasadded_ (message `/Game/DungeonsDash/_Core/BlueprintInterfaces/BPI_CardInventoryReceiver.ReceiveCard` OtherActor _cardtogive))
        (if _bwasadded_
          ;[0.9844 0.4427 0.08716 0.5 10] RECOLECCIÓN EXITOSA
          (`self.DeactivatePickup`)
          (else
            (`KismetSystemLibrary.PrintString` "Inventario lleno: pickup permanece activo" true true (struct :`R` 1.0 :`G` 0.029515 :`A` 1.0))))
        (else
          (`KismetSystemLibrary.PrintString` "No existe una carta válida para entregar" true true (struct :`R` 1.0 :`B` 0.080469 :`A` 1.0))))
      (else
        (`KismetSystemLibrary.PrintString` "ERROR: Other Actor NO implementa BPI_CardInventoryReceiver" true true (struct :`R` 1.0 :`G` 0.043238 :`A` 1.0))))))

(fn `DeactivatePickup`
  ;[0.9844 0.4427 0.08716 0.5 10] MARCAR PICKUP COMO RECOGIDO
  (set `self.bIsActive` false)
  ;[0.9844 0.4427 0.08716 0.5 10] OCULTAR PICKUP Y BLOQUEAR NUEVAS RECOLECCIONES
  (`SceneComponent.SetVisibility` (`self.PickupMesh`) false false)
  (`PrimitiveComponent.SetCollisionEnabled` (`self.SphereCollision`) "NoCollision")
  ;[0.9844 0.7478 0.1258 0.5 10] PROGRAMAR RESPAWN
  (if (`self.bCanRespawn`)
    (`KismetSystemLibrary.K2_SetTimerDelegate` (`|CreateDelegate` :!event `RespawnPickup`) (`self.RespawnTime`))))

(fn `GetCardToGive`
  (returns (CardToGive :type "/Game/DungeonsDash/_Core/Data/Cards/DA_Card_Base Object Reference") (bHasValidCard :type Boolean))
  (bind _fixedcard (`self.FixedCard`))
  (bind _possiblecards (`self.PossibleCards`))
  ;[0.6375 0.1615 1 0.5 10] DECIDIR TIPO DE CARTA
  (if (`self.bGiveRandomCard`)
    ;[0.159 0.9047 0.2705 0.502 10] VALIDAR LISTA DE CARTAS ALEATORIAS
    (if (> (`KismetArrayLibrary.Array_Length` _possiblecards) 0)
      ;[0.6375 0.1615 1 0.5 10] SELECCIONAR CARTA ALEATORIA
      (bind _output_get (set `self.SelectedRandomCard` (`KismetArrayLibrary.Array_Random` _possiblecards)))
      (`/Engine/EditorBlueprintResources/StandardMacros.IsValid` _output_get
        (:`Is Valid`
          (return (`self.SelectedRandomCard`) true))
        (:`Is Not Valid`
          (return null false)))
      (else
        ;[0.7552 0 0 0.5 10] ERROR DE CONFIGURACIÓN: ARRAY VACÍO
        (`KismetSystemLibrary.PrintString` "Pickup aleatorio sin PossibleCards" true true (struct :`R` 1.0 :`G` 0.181103 :`A` 1.0))
        (return null false)))
    (else
      ;[0.6375 0.1615 1 0.5 11] ENTREGAR CARTA FIJA
      (`/Engine/EditorBlueprintResources/StandardMacros.IsValid` _fixedcard
        (:`Is Valid`
          (return _fixedcard true))
        (:`Is Not Valid`
          ;[0.7552 0 0 0.5 10] ERROR DE CONFIGURACIÓN: FIXED CARD VACÍA
          (`KismetSystemLibrary.PrintString` "Pickup sin FixedCard configurada" true true (struct :`R` 1.0 :`G` 0.181103 :`A` 1.0))
          (return null false))))))

(fn `ReceiveCard`
  (params (CardData :type "/Game/DungeonsDash/_Core/Data/Cards/DA_Card_Base Object Reference"))
  (returns (`bWasAdded ` :type Boolean))
  (return false))

(fn `RespawnPickup`
  ;[0.9844 0.4427 0.08716 0.5 10] MOSTRAR PICKUP NUEVAMENTE
  (`SceneComponent.SetVisibility` (`self.PickupMesh`) true false)
  ;[0.159 0.9047 0.2705 0.502 10] REACTIVAR RECOLECCIÓN
  (set `self.bIsActive` true)
  (`PrimitiveComponent.SetCollisionEnabled` (`self.SphereCollision`) "QueryOnly"))

(fn `UserConstructionScript`)